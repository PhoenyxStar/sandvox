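; CameraFocus is a camera Blueprint that keeps its CameraComponent aimed at the first player's pawn.
; BeginPlay stores that pawn as TargetActor, and each Tick rotates the component's world rotation with FindLookAtRotation toward the pawn's location, without interpolation.
; Tick also calls UpdateCameraDistance, but that function is empty, so the Blueprint makes no distance adjustment.
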(event `self.ReceiveBeginPlay`
  (set `self.TargetActor` (`GameplayStatics.GetPlayerPawn` 0)))

(event `self.ReceiveTick`
  (params (DeltaSeconds :type "Float (single-precision)"))
  (`self.UpdateCameraLook`)
  (`self.UpdateCameraDistance`))

(event `UpdateCameraLook`
  (bind _cameracomponent (`self.CameraComponent`))
  (`SceneComponent.K2_SetWorldRotation` _cameracomponent (`KismetMathLibrary.FindLookAtRotation` (`SceneComponent.K2_GetComponentLocation` _cameracomponent) (`self.K2_GetActorLocation` (`self.TargetActor`))) false false))

(fn `UpdateCameraDistance`)

(fn `UserConstructionScript`)